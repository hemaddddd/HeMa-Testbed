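; BP_RollBall is a physics-driven ball that the player moves with WASD and lifts with Space.
; Each Tick polls player controller 0's keys and adds large world-axis forces to Sphere, unscaled by mass.
; Space pushes upward for as long as it is held, with no ground check.
; The Hit event checks the other actor for a "None" tag but does nothing, as its DestroyActor node is disconnected.
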(event `self.ReceiveTick`
  (params (DeltaSeconds :type "Float (single-precision)"))
  (`|ExecutionSequence`
    (:`then_0`
      (if (`PlayerController.IsInputKeyDown` (`GameplayStatics.GetPlayerController` 0) "W")
        (`PrimitiveComponent.AddForce` (`self.Sphere`) (9000000.0 0.0 0.0) "None" false)))
    (:`then_1`
      (if (`PlayerController.IsInputKeyDown` (`GameplayStatics.GetPlayerController` 0) "D")
        (`PrimitiveComponent.AddForce` (`self.Sphere`) (0.0 9000000.0 0.0) "None" false)))
    (:`then_2`
      (if (`PlayerController.IsInputKeyDown` (`GameplayStatics.GetPlayerController` 0) "S")
        (`PrimitiveComponent.AddForce` (`self.Sphere`) (-9000000.0 0.0 0.0) "None" false)))
    (:`then_3`
      (if (`PlayerController.IsInputKeyDown` (`GameplayStatics.GetPlayerController` 0) "A")
        (`PrimitiveComponent.AddForce` (`self.Sphere`) (0.0 -9000000.0 0.0) "None" false)))
    (:`then_4`
      (if (`PlayerController.IsInputKeyDown` (`GameplayStatics.GetPlayerController` 0) "SpaceBar")
        (`PrimitiveComponent.AddForce` (`self.Sphere`) (0.0 0.0 10000000.0) "None" false)))))

(event `self.ReceiveHit`
  (params (MyComp :type "PrimitiveComponent Object Reference") (Other :type "Actor Object Reference") (OtherComp :type "PrimitiveComponent Object Reference") (bSelfMoved :type Boolean) (HitLocation :type "Vector Structure") (HitNormal :type "Vector Structure") (NormalImpulse :type "Vector Structure") (Hit :type "HitResult Structure (by ref)"))
  (if (`self.ActorHasTag` Other "None")
    _))

(fn `UserConstructionScript`)